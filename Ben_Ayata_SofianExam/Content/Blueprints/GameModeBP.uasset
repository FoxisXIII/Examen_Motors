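; GameModeBP is a Game Mode Blueprint that stores the player's Life and Hearts values.
; BeginPlay initializes Life, while Hearts is not set in any graph and changes only through increaseHearts, which adds one.
; The getLife and getHearts functions return the current values, and Tick and the construction script are empty.
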(event `self.ReceiveBeginPlay`
  (set `self.life` 100.0))

(fn `getHearts`
  (returns (hearts :type Integer))
  (return (`self.hearts`)))

(fn `getLife`
  (returns (life :type "Float (double-precision)"))
  (return (`self.life`)))

(fn `increaseHearts`
  (set `self.hearts` (+ (`self.hearts`) 1)))

(fn `UserConstructionScript`)